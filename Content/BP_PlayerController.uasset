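; Player controller that runs click-to-talk NPC dialogue and click-to-pickup items through dialogue and inventory widgets.
; BeginPlay creates both widgets, opens dialogue with Game and UI input, and binds NPC clicks, with item binding nested inside the NPC loop.
; Clicks pass dialogue type or item type to the widgets, hiding picked-up items.
; Keys page or close dialogue and pop up inventory, with viewport checks preventing overlapping interactions.
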(event `self.ReceiveBeginPlay`
  (bind _returnvalue (`|CreateWidget` "/Game/WB_Inventory.WB_Inventory_C" self))
  (bind _output_get (set `self.InventoryUI` _returnvalue))
  (`BasePopup.Enable` _output_get)
  (`BasePopup.Disable` _output_get)
  (bind _returnvalue_2 (`|CreateWidget` "/Game/WB_Dialogue.WB_Dialogue_C" self))
  (bind _output_get_2 (set `self.DialogueUI` _returnvalue_2))
  (`BasePopup.Enable` _output_get_2)
  (`WidgetBlueprintLibrary.SetInputMode_GameAndUIEx` self _output_get_2)
  (bind _outactors (`GameplayStatics.GetAllActorsOfClass` "/Script/FlawlessAbbeyJulian.BaseNPC"))
  (for _array_element _outactors
    (add `self.OnClicked` _array_element (delegate `EventTalkTrigger`))
    (bind _outactors_2 (`GameplayStatics.GetAllActorsOfClass` "/Script/FlawlessAbbeyJulian.BaseItem"))
    (for _array_element_2 _outactors_2
      (add `self.OnClicked` _array_element_2 (delegate `EventPickup`)))))

(event `Key|SpaceBar`
  (params (Key :type "Key Structure"))
  (:`Pressed`
    (`/Game/WB_Dialogue.PageJump` (`self.DialogueUI`))))

(event `Key|Enter`
  (params (Key :type "Key Structure"))
  (:`Pressed`
    (bind _dialogueui (`self.DialogueUI`)
      (:`then`
        (`BasePopup.Disable` _dialogueui))
      (:`else`))))

(event `Key|I`
  (params (Key :type "Key Structure"))
  (:`Released`
    (bind _inventoryui (`self.InventoryUI`)
      (:`then`
        (if (not (`Widget.IsInViewport` (`self.DialogueUI`)))
          (`BasePopup.Popup` _inventoryui)))
      (:`else`))))

(event `EventTalkTrigger`
  (params (TouchedActor :type "Actor Object Reference") (ButtonPressed :type "Key Structure" :default "None"))
  (bind _asbase_npc (cast `BaseNPC` TouchedActor))
  (bind _dialogueui (`self.DialogueUI`)
    (:`then`
      (if (and (not (`Widget.IsInViewport` (`self.InventoryUI`))) (not (`Widget.IsInViewport` _dialogueui)))
        (set `/Game/WB_Dialogue.RowDialogueType` (`BaseNPC.DialogueType` _asbase_npc) _dialogueui)
        (`BasePopup.Enable` _dialogueui)))
    (:`else`)))

(event `EventPickup`
  (params (TouchedActor :type "Actor Object Reference") (ButtonPressed :type "Key Structure" :default "None"))
  (bind _asbase_item (cast `BaseItem` TouchedActor))
  (bind _inventoryui (`self.InventoryUI`)
    (:`then`
      (if (and (not (`Widget.IsInViewport` (`self.DialogueUI`))) (not (`Widget.IsInViewport` _inventoryui)))
        (`BaseItem.Hidde` _asbase_item)
        (`/Game/WB_Inventory.EventAddItem` _inventoryui (`BaseItem.ItemType` _asbase_item))))
    (:`else`)))

(fn `UserConstructionScript`)