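; Base item actor that can be rotated and zoomed from UI input, with a SceneCaptureComponent2D viewing its mesh, apparently for item inspection.
; Movement input adds local yaw and pitch to the mesh, while zoom slides the capture component along local X only within a limit around its starting offset.
; Rotation and zoom reset to values cached at BeginPlay, and hiding relocates the actor to a set position instead of changing visibility.
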(event `self.ReceiveBeginPlay`
  (bind _relativelocation_x (`KismetMathLibrary.BreakVector` (`SceneComponent.RelativeLocation` (`self.SceneCaptureComponent2D`))))
  (set `self.DefaultRotation` (`SceneComponent.RelativeRotation` (`self.ItemMesh`)))
  (set `self.DefaultZoom` _relativelocation_x))

(event `EventUpdateZoom`
  (params (ZoomOffset :type "Float (double-precision)"))
  (bind _scenecapturecomponent2d (`self.SceneCaptureComponent2D`)
    (:`then`
      (bind _valid (`self.ValidZoomOffset` ZoomOffset))
      (if _valid
        (`SceneComponent.K2_AddLocalOffset` _scenecapturecomponent2d (`KismetMathLibrary.MakeVector` ZoomOffset) false false)))
    (:`else`)))

(event `EventUpdateRotation`
  (params (MovementUI :type "Vector2D Structure"))
  (bind _itemmesh (`self.ItemMesh`)
    (:`then`
      (`SceneComponent.K2_AddLocalRotation` _itemmesh (`KismetMathLibrary.MakeRotator` 0.0 MovementUI_Y MovementUI_X) false false))
    (:`else`)))

(event `EventResetRotation`
  (bind _itemmesh (`self.ItemMesh`)
    (:`then`
      (`SceneComponent.K2_SetRelativeRotation` _itemmesh (`self.DefaultRotation`) false false))
    (:`else`)))

(event `EventResetZoom`
  (bind _scenecapturecomponent2d (`self.SceneCaptureComponent2D`)
    (:`then`
      (bind (_relativelocation_x _relativelocation_y _relativelocation_z) (`KismetMathLibrary.BreakVector` (`SceneComponent.RelativeLocation` _scenecapturecomponent2d)))
      (`SceneComponent.K2_SetRelativeLocation` _scenecapturecomponent2d (`KismetMathLibrary.MakeVector` (`self.DefaultZoom`) _relativelocation_y _relativelocation_z) false false))
    (:`else`)))

(event `EventHidde`
  (`self.K2_SetActorLocation` (`self.HiddePosition`)))

(fn `UserConstructionScript`)

(fn `ValidZoomOffset`
  (params (ZoomOffsetOffset :type "Float (double-precision)"))
  (returns (Valid :type Boolean))
  (bind _relativelocation_x (`KismetMathLibrary.BreakVector` (`SceneComponent.RelativeLocation` (`self.SceneCaptureComponent2D`))))
  (return (< (`KismetMathLibrary.Abs` (+ ZoomOffsetOffset (- _relativelocation_x (`self.DefaultZoom`)))) (`self.ZoomLimit`))))